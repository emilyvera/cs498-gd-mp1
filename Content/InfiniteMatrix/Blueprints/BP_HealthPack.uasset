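; BP_HealthPack is a pickup that gives the player an extra life when touched.
; On BeginPlay it caches the game mode as GM_Tutorial.
; When BP_Player overlaps the HealthIcon component, it increments the game mode's Lives if below three, then destroys itself, even when no life is added.
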(event `self.ReceiveBeginPlay`
  (bind _asgm_tutorial (cast `/Game/InfiniteMatrix/Blueprints/GM_Tutorial` (`GameplayStatics.GetGameMode`)))
  (set `self.GameMode` _asgm_tutorial))

(event `self.HealthIcon.OnComponentBeginOverlap`
  (params (OverlappedComponent :type "PrimitiveComponent Object Reference") (OtherActor :type "Actor Object Reference") (OtherComp :type "PrimitiveComponent Object Reference") (OtherBodyIndex :type Integer) (bFromSweep :type Boolean) (SweepResult :type "HitResult Structure (by ref)"))
  (bind _gamemode (`self.GameMode`))
  (bind _lives (`/Game/InfiniteMatrix/Blueprints/GM_Tutorial.Lives` _gamemode))
  (cast `/Game/InfiniteMatrix/Blueprints/BP_Player` OtherActor)
  (if (< _lives 3)
    (set `/Game/InfiniteMatrix/Blueprints/GM_Tutorial.Lives` (+ _lives 1) _gamemode))
  (`self.K2_DestroyActor`))

(fn `UserConstructionScript`)