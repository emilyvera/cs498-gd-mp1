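; BP_Projectile is a projectile in InfiniteMatrix that flies along world X, staying faster than the game's forward speed.
; It caches GM_Tutorial on BeginPlay, then each Tick makes a swept move at that game mode's ForwardSpeed plus a fixed boost.
; Overlapping any actor other than BP_Player destroys it.
; The Projectile component's own overlap event casts to BP_Player but takes no further action.
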(event `self.ReceiveBeginPlay`
  (bind _asgm_tutorial (cast `/Game/InfiniteMatrix/Blueprints/GM_Tutorial` (`GameplayStatics.GetGameMode`)))
  (set `self.GameMode` _asgm_tutorial))

(event `self.ReceiveActorBeginOverlap`
  (params (OtherActor :type "Actor Object Reference"))
  (cast `/Game/InfiniteMatrix/Blueprints/BP_Player` OtherActor
    (:`CastFailed`
      (`self.K2_DestroyActor`))))

(event `self.ReceiveTick`
  (params (DeltaSeconds :type "Float (single-precision)"))
  (`self.K2_AddActorWorldOffset` (`KismetMathLibrary.MakeVector` (* DeltaSeconds (+ (`/Game/InfiniteMatrix/Blueprints/GM_Tutorial.ForwardSpeed` (`self.GameMode`)) 750.0))) true))

(event `self.Projectile.OnComponentBeginOverlap`
  (params (OverlappedComponent :type "PrimitiveComponent Object Reference") (OtherActor :type "Actor Object Reference") (OtherComp :type "PrimitiveComponent Object Reference") (OtherBodyIndex :type Integer) (bFromSweep :type Boolean) (SweepResult :type "HitResult Structure (by ref)"))
  (cast `/Game/InfiniteMatrix/Blueprints/BP_Player` OtherActor))

(fn `UserConstructionScript`)